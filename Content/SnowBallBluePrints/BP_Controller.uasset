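; Player controller for a snowball game that rolls the player's physics ball with WASD and handles mouse look.
; Tick polls the keys and applies mass-independent force to BPPlayer's Ball along the camera's forward and right vectors.
; Mouse Y feeds inverted pitch, while Mouse X passes zero to yaw.
; The cast that would set BPPlayer from the controlled pawn is disconnected, so this graph never assigns that reference.
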(event EventBeginPlay)

(event EventTick
  (params (DeltaSeconds :type Float%20%28single-precision%29))
  (bind _bp_player (Variables|Default|GetBP%20Player))
  (bind _bp_player_2 (Variables|Default|GetBP%20Player))
  (bind _bp_player_3 (Variables|Default|GetBP%20Player))
  (bind _bp_player_4 (Variables|Default|GetBP%20Player))
  ;[1 1 1] Ball Foward
  (Utilities|FlowControl|Sequence
    (:then_0
      (if (Game|Player|IsInputKeyDown "W")
        (Physics|AddForce (Variables|/Game/SnowBallBluePrints/BP_Player.BP_Player_C|GetBall _bp_player_2) (* (Math|Vector|GetForwardVector (Variables|/Game/SnowBallBluePrints/BP_Player.BP_Player_C|GetCamera _bp_player_2)) 1e+03) "None" true)))
    (:then_1
      ;[1 1 1] Ball Backward
      (if (Game|Player|IsInputKeyDown "S")
        (Physics|AddForce (Variables|/Game/SnowBallBluePrints/BP_Player.BP_Player_C|GetBall _bp_player_3) (* (Math|Vector|GetForwardVector (Variables|/Game/SnowBallBluePrints/BP_Player.BP_Player_C|GetCamera _bp_player_3)) -1e+03) "None" true)))
    (:then_2
      ;[1 1 1] Ball Left
      (if (Game|Player|IsInputKeyDown "A")
        (Physics|AddForce (Variables|/Game/SnowBallBluePrints/BP_Player.BP_Player_C|GetBall _bp_player_4) (* (Math|Vector|GetRightVector (Variables|/Game/SnowBallBluePrints/BP_Player.BP_Player_C|GetCamera _bp_player_4)) -1e+03) "None" true)))
    (:then_3
      ;[1 1 1] Ball right
      (if (Game|Player|IsInputKeyDown "D")
        (Physics|AddForce (Variables|/Game/SnowBallBluePrints/BP_Player.BP_Player_C|GetBall _bp_player) (* (Math|Vector|GetRightVector (Variables|/Game/SnowBallBluePrints/BP_Player.BP_Player_C|GetCamera _bp_player)) 1e+03) "None" true)))))

(event Input|MouseEvents|MouseX
  (params (AxisValue :type Float%20%28single-precision%29))
  (Class|PlayerController|AddYawInput 0.0))

(event Input|MouseEvents|MouseY
  (params (AxisValue :type Float%20%28single-precision%29))
  (Class|PlayerController|AddPitchInput (* AxisValue -1.0)))

(fn ConstructionScript)